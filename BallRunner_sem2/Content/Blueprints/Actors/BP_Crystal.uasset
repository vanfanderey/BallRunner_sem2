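; BP_Crystal is a crystal actor that flies into the player and disappears when the player pawn overlaps its sphere.
; The overlap plays a timeline whose Movement and Scale tracks feed two helper functions, and the actor is destroyed when it finishes.
; Each update lerps from the current transform toward the player's live location and zero scale, so the motion homes in and compounds over frames.
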(event `self.Sphere.OnComponentBeginOverlap`
  (params (OverlappedComponent :type "PrimitiveComponent Object Reference") (OtherActor :type "Actor Object Reference") (OtherComp :type "PrimitiveComponent Object Reference") (OtherBodyIndex :type Integer) (bFromSweep :type Boolean) (SweepResult :type "HitResult Structure (by ref)"))
  (if (== OtherActor (`GameplayStatics.GetPlayerPawn` 0))
    (bind (_direction _movement _scale) (`Timeline|TL_CrystalMovement`)
      (:`Update`
        (`self.Location` _movement)
        (`self.Scale` _scale))
      (:`Finished`
        (`self.K2_DestroyActor`)))))

(fn `Location`
  (params (Alpha :type "Float (double-precision)"))
  (`self.K2_SetActorLocation` (`KismetMathLibrary.VLerp` (`self.K2_GetActorLocation`) (`self.K2_GetActorLocation` (`GameplayStatics.GetPlayerPawn` 0)) Alpha)))

(fn `Scale`
  (params (Alpha :type "Float (double-precision)"))
  (`self.SetActorScale3D` (`KismetMathLibrary.VLerp` (`self.GetActorScale3D`) (0.0 0.0 0.0) Alpha)))

(fn `UserConstructionScript`)